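; A book actor made of skeletal mesh page components that can be picked up and dropped through BP_MotionController.
; BeginPlay gathers the covers and every page into an ordered PageComponents array, which only an unconnected debug print reads here.
; Pickup turns off physics and attaches the root to the given component, keeping world transform.
; Drop restores physics and detaches it, with both events updating the PickedUp flag.
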(event EventBeginPlay
  ;[1 1 1] Creates array of all the skeletal mesh actor components (ie. all the pages of the book)
  (Variables|Default|SetpageComponents (Utilities|Array|MakeArray (Variables|Default|Getcover_page) (Variables|Default|Getpage_01_02) (Variables|Default|Getpage_03_04) (Variables|Default|Getpage_05_06) (Variables|Default|Getpage_07_08) (Variables|Default|Getpage_09_10) (Variables|Default|Getpage_11_12) (Variables|Default|Getpage_13_14) (Variables|Default|Getpage_15_16) (Variables|Default|Getpage_17_18) (Variables|Default|Getpage_19_20) (Variables|Default|Getpage_21_22) (Variables|Default|Getpage_23_24) (Variables|Default|Getpage_25_26) (Variables|Default|Getpage_27_28) (Variables|Default|Getpage_29_30) (Variables|Default|Getpage_31_32) (Variables|Default|Getpage_33_34) (Variables|Default|Getpage_35_36) (Variables|Default|Getpage_37_38) (Variables|Default|Getpage_39_40) (Variables|Default|Getpage_41_42) (Variables|Default|Getpage_43_44) (Variables|Default|Getpage_45_46) (Variables|Default|Getpage_47_48) (Variables|Default|Getpage_49_50) (Variables|Default|Getpage_51_52) (Variables|Default|Getpage_53_54) (Variables|Default|Getpage_55_56) (Variables|Default|Getpage_57_58) (Variables|Default|Getpage_59_60) (Variables|Default|Getpage_61_62) (Variables|Default|Getpage_63_64) (Variables|Default|Getback_page))))

(event Collision|EventActorBeginOverlap
  (params (OtherActor :type Actor%20Object%20Reference)))

(event EventTick
  (params (DeltaSeconds :type Float%20%28single-precision%29)))

(event EventPickup
  (params (AttachTo :type Scene%20Component%20Object%20Reference))
  (Physics|SetSimulatePhysics (Variables|SkeletalMeshActor|GetSkeletalMeshComponent) false)
  (Transformation|AttachComponentToComponent (VehicleSound|GetRootComponent) AttachTo "None" "KeepWorld" "KeepWorld" "KeepWorld" false)
  (Variables|Default|Setpicked_up true))

(event EventDrop
  (Physics|SetSimulatePhysics (Variables|SkeletalMeshActor|GetSkeletalMeshComponent) true)
  (Transformation|DetachFromActor "KeepWorld" "KeepWorld" "KeepWorld")
  (Variables|Default|Setpicked_up false))

(fn ConstructionScript)